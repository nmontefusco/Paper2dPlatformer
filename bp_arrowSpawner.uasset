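; Arrow trap actor that moves along the vertical axis while firing arrows on a repeating timer.
; On BeginPlay it stores its start position, starts the looping Fire timer and plays a timeline that lerps its height by the Speed variable, which acts as a distance offset.
; Each Fire call spawns a Bp_arrow at the SpawnPoint transform and plays a quiet crossbow shot sound.
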(event `self.ReceiveBeginPlay`
  (bind (_startpos_x _startpos_y _startpos_z) (`KismetMathLibrary.BreakVector` (`self.StartPos`)))
  (set `self.StartPos` (`self.K2_GetActorLocation`))
  (`KismetSystemLibrary.K2_SetTimer` null "Fire" 1.0 true)
  (bind (_direction _move) (`Timeline|Movement_Timeline` :!via `PlayFromStart`)
    (:`Update`
      (`self.K2_SetActorLocation` (`KismetMathLibrary.VLerp` (`self.StartPos`) (`KismetMathLibrary.MakeVector` _startpos_x _startpos_y (+ _startpos_z (`self.Speed`))) _move)))))

(event `Fire`
  (`|SpawnActorFromClass` "/Game/BluePrint/bp_arrow.bp_arrow_C" (`SceneComponent.K2_GetComponentToWorld` (`self.SpawnPoint`)) "Undefined" "OverrideRootScale" null null)
  (`GameplayStatics.PlaySoundAtLocation` "/Game/Sound/bow_crossbow_arrow_shoot_type3_03.bow_crossbow_arrow_shoot_type3_03" (`self.K2_GetActorLocation`) (struct) 0.1))

(fn `UserConstructionScript`)