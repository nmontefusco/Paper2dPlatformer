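; Ladder actor that lets the Player climb while inside its Box trigger.
; The construction script stacks collision-free Paper2D sprites at a fixed spacing between LadderBottom and LadderTop, then scales and offsets the Box vertically from that height.
; Box overlap sets the Player's IsCanClimb flag, and leaving clears it and calls ClimbingEnd.
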(event `self.Box.OnComponentBeginOverlap`
  (params (OverlappedComponent :type "PrimitiveComponent Object Reference") (OtherActor :type "Actor Object Reference") (OtherComp :type "PrimitiveComponent Object Reference") (OtherBodyIndex :type Integer) (bFromSweep :type Boolean) (SweepResult :type "HitResult Structure (by ref)"))
  (bind _asplayer (cast `/Game/BluePrint/Player` OtherActor))
  (set `/Game/BluePrint/Player.is_CanClimb` true _asplayer))

(event `self.Box.OnComponentEndOverlap`
  (params (OverlappedComponent :type "PrimitiveComponent Object Reference") (OtherActor :type "Actor Object Reference") (OtherComp :type "PrimitiveComponent Object Reference") (OtherBodyIndex :type Integer))
  (bind _asplayer (cast `/Game/BluePrint/Player` OtherActor))
  (set `/Game/BluePrint/Player.is_CanClimb` false _asplayer)
  (`/Game/BluePrint/Player.ClimbingEnd` _asplayer))

(fn `UserConstructionScript`
  (bind _box (`self.Box`))
  (bind _rangeoffset (`self.RangeOffset`))
  (bind (_returnvalue_x _returnvalue_y _returnvalue_z) (`KismetMathLibrary.BreakVector` (- (`self.ladderTop`) (`self.ladderBottom`))))
  (bind _returnvalue (/ _returnvalue_z 2.0))
  (for _index (range (+ (`KismetMathLibrary.FTrunc` (/ _returnvalue_z _rangeoffset)) 1))
    (bind _returnvalue_2 (`AddComponent|NODE_AddPaperSpriteComponent-0` :`RelativeTransform` (`KismetMathLibrary.MakeTransform` (`KismetMathLibrary.MakeVector` 0.0 0.0 (* _index _rangeoffset)))))
    (`PaperSpriteComponent.SetSprite` _returnvalue_2 (`self.ladderSprite`))
    (`PrimitiveComponent.SetCollisionEnabled` _returnvalue_2 "NoCollision"))
  (`SceneComponent.SetRelativeScale3D` _box (`KismetMathLibrary.MakeVector` 0.0 0.0 _returnvalue))
  (`SceneComponent.K2_AddRelativeLocation` _box (`KismetMathLibrary.MakeVector` 0.0 0.0 _returnvalue) false false))