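; Projectile actor, scaled to a tenth in its construction script, that kills enemies on impact and wobbles when it hits anything else.
; A collision hit on a bp_enemy applies damage, then destroys both enemy and projectile immediately.
; Other hits, and the Hit event, play a wooden sound and start a timeline that wobbles the yaw, disables collision and destroys the projectile after a delay.
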(event `self.Collision.OnComponentHit`
  (params (HitComponent :type "PrimitiveComponent Object Reference") (OtherActor :type "Actor Object Reference") (OtherComp :type "PrimitiveComponent Object Reference") (NormalImpulse :type "Vector Structure") (Hit :type "HitResult Structure (by ref)"))
  (bind _asbp_enemy (cast `/Game/BluePrint/bp_enemy` OtherActor)
    (:`then`
      (`GameplayStatics.ApplyDamage` _asbp_enemy 10.0 null null "/Script/Engine.DamageType")
      (`self.K2_DestroyActor` _asbp_enemy)
      (`self.K2_DestroyActor`))
    (:`CastFailed`
      (`GameplayStatics.PlaySound2D` "/Game/Sound/footstep_wood_run_wobble_04.footstep_wood_run_wobble_04" :!label _label)
      (bind (_direction _wobble) (`Timeline|Timeline_0` :!via `PlayFromStart`)
        (:`Update`
          (`SceneComponent.K2_SetRelativeRotation` (`self.Scene`) (`KismetMathLibrary.RLerp` (struct) (struct :`Pitch` 10.0) _wobble) false false)
          (`PrimitiveComponent.SetCollisionEnabled` (`self.Collision`) "NoCollision")
          (`KismetSystemLibrary.Delay` 4.0)
          (`self.K2_DestroyActor`))))))

(event `self.ReceiveHit`
  (params (MyComp :type "PrimitiveComponent Object Reference") (Other :type "Actor Object Reference") (OtherComp :type "PrimitiveComponent Object Reference") (bSelfMoved :type Boolean) (HitLocation :type "Vector Structure") (HitNormal :type "Vector Structure") (NormalImpulse :type "Vector Structure") (Hit :type "HitResult Structure (by ref)"))
  (goto _label))

(fn `UserConstructionScript`
  (`self.SetActorScale3D` (0.1 0.1 0.1)))