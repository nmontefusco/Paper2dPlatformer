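; Arrow projectile Blueprint that damages the player on hit or sticks with a wobble on anything else.
; A player hit applies fixed damage and destroys the arrow at once.
; Other hits play a wood sound and a Timeline that drives a small wobble rotation on the Scene component.
; The Timeline update also disables collision and starts a delay before the arrow destroys itself.
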(event `self.ReceiveHit`
  (params (MyComp :type "PrimitiveComponent Object Reference") (Other :type "Actor Object Reference") (OtherComp :type "PrimitiveComponent Object Reference") (bSelfMoved :type Boolean) (HitLocation :type "Vector Structure") (HitNormal :type "Vector Structure") (NormalImpulse :type "Vector Structure") (Hit :type "HitResult Structure (by ref)"))
  (bind _asplayer (cast `/Game/BluePrint/Player` Other)
    (:`then`
      (bind _output_get (set `self.player_bp` _asplayer))
      (`GameplayStatics.ApplyDamage` _output_get 1.0)
      (`self.K2_DestroyActor`))
    (:`CastFailed`
      (`GameplayStatics.PlaySound2D` "/Game/Sound/footstep_wood_run_wobble_04.footstep_wood_run_wobble_04")
      (bind (_direction _wobble) (`Timeline|Wobble` :!via `PlayFromStart`)
        (:`Update`
          (`SceneComponent.K2_SetRelativeRotation` (`self.Scene`) (`KismetMathLibrary.RLerp` (struct) (struct :`Pitch` 10.0) _wobble) false false)
          (`PrimitiveComponent.SetCollisionEnabled` (`self.Collision`) "NoCollision")
          (`KismetSystemLibrary.Delay` 4.0)
          (`self.K2_DestroyActor`))))))

(fn `UserConstructionScript`)